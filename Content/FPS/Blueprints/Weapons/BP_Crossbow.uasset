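; Crossbow weapon Blueprint that keeps its loaded bolt visual in step with the ammo count.
; Its HideBolt override calls the parent, then hides the first- and third-person bolt components when ActualAmmo is zero and shows them otherwise.
; The construction script only calls the parent, and leftover SetHiddenInGame nodes are disconnected in favor of SetVisibility.
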(fn ConstructionScript
  (|CallParentFunction))

(fn HideBolt
  (|CallParentFunction)
  (if (== (Variables|Default|GetActualAmmo) 0)
    (Rendering|SetVisibility (Variables|Default|GetCrossbowBoltFPP) false false)
    (Rendering|SetVisibility (Variables|Default|GetCrossbowBoltTPP) false false)
    (else
      (Rendering|SetVisibility (Variables|Default|GetCrossbowBoltFPP) true false)
      (Rendering|SetVisibility (Variables|Default|GetCrossbowBoltTPP) true false))))